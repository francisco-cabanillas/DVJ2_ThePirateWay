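; BP_Border is a rotating puzzle piece in the Isla level where one mesh is selected and checked against an answer.
; While the third-person character overlaps its capsule, RotatingMovement spins it and a looping sound plays.
; SetSelected moves an emissive material to the hit component and updates IsRight, only when the game mode's papyrus counts match and the level is uncompleted.
; RandomRotation can give StaticMesh4 a random yaw.
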(event `self.Capsule.OnComponentBeginOverlap`
  (params (OverlappedComponent :type "PrimitiveComponent Object Reference") (OtherActor :type "Actor Object Reference") (OtherComp :type "PrimitiveComponent Object Reference") (OtherBodyIndex :type Integer) (bFromSweep :type Boolean) (SweepResult :type "HitResult Structure (by ref)"))
  ;[1 1 1] Rotation
  (cast `/Game/Personaje/Blueprints/ThirdPersonCharacter` OtherActor)
  (set `RotatingMovementComponent.RotationRate` (`KismetMathLibrary.MakeRotator` 0.0 0.0 (`KismetMathLibrary.Conv_IntToDouble` (`self.RotationRate`))) (`self.RotatingMovement`))
  (`AudioComponent.Play` (`self.AudioLoop`) 0.0))

(event `self.Capsule.OnComponentEndOverlap`
  (params (OverlappedComponent :type "PrimitiveComponent Object Reference") (OtherActor :type "Actor Object Reference") (OtherComp :type "PrimitiveComponent Object Reference") (OtherBodyIndex :type Integer))
  ;[1 1 1] Rotation
  (cast `/Game/Personaje/Blueprints/ThirdPersonCharacter` OtherActor)
  (set `RotatingMovementComponent.RotationRate` (`KismetMathLibrary.MakeRotator` 0.0) (`self.RotatingMovement`))
  (`AudioComponent.Stop` (`self.AudioLoop`)))

(fn `CanInteract`
  (bind _asthird_person_game_mode (cast `/Game/Personaje/Blueprints/ThirdPersonGameMode` (`GameplayStatics.GetGameMode`)))
  (set `self.IsAvailable` (and (== (`/Game/Personaje/Blueprints/ThirdPersonGameMode.TotalPapyrus` _asthird_person_game_mode) (`/Game/Personaje/Blueprints/ThirdPersonGameMode.PapyrusLeft` _asthird_person_game_mode)) (not (`/Game/Personaje/Blueprints/ThirdPersonGameMode.IslaLevelCompleted` _asthird_person_game_mode)))))

(fn `Random Rotation`
  (`SceneComponent.K2_SetWorldRotation` (`self.StaticMesh4`) (`KismetMathLibrary.MakeRotator` 0.0 0.0 (`KismetMathLibrary.Conv_IntToDouble` (`KismetMathLibrary.RandomInteger` 350))) false false))

(fn `SetSelected`
  (params (HitComponent :type "PrimitiveComponent Object Reference"))
  (bind _selected (`self.Selected`))
  (`self.CanInteract`)
  (if (`self.IsAvailable`)
    (`/Engine/EditorBlueprintResources/StandardMacros.IsValid` _selected
      (:`Is Valid`
        (`PrimitiveComponent.SetMaterialByName` _selected "Object001" (`self.Non-emissive`))
        (set `self.Selected` null))
      (:`Is Not Valid`
        _))
    (`/Engine/EditorBlueprintResources/StandardMacros.IsValid` HitComponent
      (:`Is Valid`
        (`PrimitiveComponent.SetMaterialByName` HitComponent "Object001" (`self.emissive`))
        (set `self.Selected` HitComponent))
      (:`Is Not Valid`
        (set `self.Selected` null)))
    (if (== (`self.Answer`) (`self.Selected`))
      (set `self.IsRight` true)
      (else
        (set `self.IsRight` false)))))

(fn `UserConstructionScript`)