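; BP_Random_Item is a placeable spawn point that randomly chooses its child actor class on BeginPlay, with Papyrus as one option.
; Before rolling, it narrows the random range: excluding Papyrus once PapyrusMax exist, or forcing it when undecided points equal the remaining shortfall.
; It tracks resolved points through a ThirdPersonGameMode counter, so random placement still aims to meet the Papyrus quota exactly.
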(event `self.ReceiveBeginPlay`
  ;[1 1 1] Generate Elements
  (`self.PapyrusMaxCreated`)
  (`self.PapyrusNeedCreated`)
  (`ChildActorComponent.SetChildActorClass` (`self.ChildActor`) (select `int` (`KismetMathLibrary.RandomIntegerInRange` (`self.MinItemTypes`) (`self.MaxItemTypes`)) :`0` (`self.Papyrus`) :`1` null))
  (bind _asthird_person_game_mode (cast `/Game/Personaje/Blueprints/ThirdPersonGameMode` (`GameplayStatics.GetGameMode`)))
  (bind _result (`/Engine/EditorBlueprintResources/StandardMacros.IncrementInt` (`/Game/Personaje/Blueprints/ThirdPersonGameMode.TotalRandomItemCreated` _asthird_person_game_mode))
    (:`  `
      (set `/Game/Personaje/Blueprints/ThirdPersonGameMode.TotalRandomItemCreated` _result _asthird_person_game_mode))))

(fn `PapyrusMaxCreated`
  (bind _outactors (`GameplayStatics.GetAllActorsOfClass` "/Game/Isla/Blueprints/BP_Papyrus.BP_Papyrus_C"))
  (if (== (`KismetArrayLibrary.Array_Length` _outactors) (`self.PapyrusMax`))
    (set `self.MinItemTypes` 1)))

(fn `PapyrusNeedCreated`
  (bind _asthird_person_game_mode (cast `/Game/Personaje/Blueprints/ThirdPersonGameMode` (`GameplayStatics.GetGameMode`)))
  (bind _outactors (`GameplayStatics.GetAllActorsOfClass` "BP_Random_Item_C"))
  (bind _outactors_2 (`GameplayStatics.GetAllActorsOfClass` "/Game/Isla/Blueprints/BP_Papyrus.BP_Papyrus_C"))
  (if (== (- (`self.PapyrusMax`) (`KismetArrayLibrary.Array_Length` _outactors_2)) (- (`KismetArrayLibrary.Array_Length` _outactors) (`/Game/Personaje/Blueprints/ThirdPersonGameMode.TotalRandomItemCreated` _asthird_person_game_mode)))
    (set `self.MaxItemTypes` 0)))

(fn `UserConstructionScript`)