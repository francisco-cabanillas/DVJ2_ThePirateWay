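; BP_Papyrus is a papyrus pickup that starts a platform mission when the player character collects it.
; Overlapping its box plays the pickup sound for any actor, then, if that actor is ThirdPersonCharacter, calls StartPlatformMission and PapiroFound and destroys the papyrus.
; On BeginPlay it counts existing BP_Papyrus actors and sets Value to "Oeste" for two or fewer, otherwise "Este".
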(event `self.Box.OnComponentBeginOverlap`
  (params (OverlappedComponent :type "PrimitiveComponent Object Reference") (OtherActor :type "Actor Object Reference") (OtherComp :type "PrimitiveComponent Object Reference") (OtherBodyIndex :type Integer) (bFromSweep :type Boolean) (SweepResult :type "HitResult Structure (by ref)"))
  ;[1 1 1] Get Papyrus
  (`GameplayStatics.PlaySound2D` "/Game/Audio/Isla/fx_recogerpapiro_Cue.fx_recogerpapiro_Cue" 1.0 1.0 0.0 null null false)
  (bind _asthird_person_character (cast `/Game/Personaje/Blueprints/ThirdPersonCharacter` OtherActor))
  (`/Game/Personaje/Blueprints/ThirdPersonCharacter.StartPlatformMission` _asthird_person_character)
  (`/Game/Personaje/Blueprints/ThirdPersonCharacter.PapiroFound` _asthird_person_character)
  (`self.K2_DestroyActor`))

(event `self.ReceiveBeginPlay`
  ;[1 1 1] Set Papyrus Value
  (bind _outactors (`GameplayStatics.GetAllActorsOfClass` "BP_Papyrus_C"))
  (if (<= (`KismetArrayLibrary.Array_Length` _outactors) 2)
    (set `self.Value` "Oeste")
    (else
      (set `self.Value` "Este"))))

(fn `UserConstructionScript`)