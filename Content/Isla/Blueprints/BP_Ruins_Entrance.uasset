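; Ruins entrance doors on the island level, gated by a papyrus mission and then a rock mission, that lead into the Ruins level.
; Tick polls actor counts: no BP_Papyrus left reveals the door carving, and every BP_Border being IsRight lights the emissive via dynamic materials.
; With both done, an overlap binds the player's interact input to a timeline that swings the doors open.
; A separate trigger box loads Ruins.
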(event `self.ReceiveTick`
  (params (DeltaSeconds :type "Float (single-precision)"))
  (bind _materialdynamicizq (`self.MaterialDynamicIzq`))
  (bind _materialdynamicder (`self.MaterialDynamicDer`))
  (if (`self.MisionPapyrusCompleted`)
    (if (not (`self.LevelCompleted`))
      (bind _outactors (`GameplayStatics.GetAllActorsOfClass` "/Game/Isla/Blueprints/BP_Border.BP_Border_C"))
      (for _array_element _outactors
        (if (`/Game/Isla/Blueprints/BP_Border.IsRight` _array_element)
          (bind _result (`/Engine/EditorBlueprintResources/StandardMacros.IncrementInt` (`self.RocksCompleted`))
            (:`  `
              (set `self.RocksCompleted` _result)))))
      (bind _output_get (set `self.MisionRocksCompleted` (== (`self.RocksCompleted`) (`KismetArrayLibrary.Array_Length` _outactors))))
      (set `self.RocksCompleted` 0)
      (if _output_get
        (`MaterialInstanceDynamic.SetScalarParameterValue` _materialdynamicizq "Emissive" 1.0)
        (`MaterialInstanceDynamic.SetScalarParameterValue` _materialdynamicder "Emissive" 1.0)
        (else
          (`MaterialInstanceDynamic.SetScalarParameterValue` _materialdynamicizq "Emissive" 0.0)
          (`MaterialInstanceDynamic.SetScalarParameterValue` _materialdynamicder "Emissive" 0.0))))
    (else
      (bind _outactors_2 (`GameplayStatics.GetAllActorsOfClass` "/Game/Isla/Blueprints/BP_Papyrus.BP_Papyrus_C"))
      (bind _returnvalue (`KismetArrayLibrary.Array_Length` _outactors_2))
      (if (!= _returnvalue (`self.PapyrusFound`))
        (bind _output_get_2 (set `self.PapyrusFound` _returnvalue))
        (bind _asthird_person_game_mode (cast `/Game/ThirdPersonBP/Blueprints/ThirdPersonGameMode` (`GameplayStatics.GetGameMode`)))
        (set `/Game/ThirdPersonBP/Blueprints/ThirdPersonGameMode.PapyrusLeft` (- 3 _output_get_2) _asthird_person_game_mode)
        (if (== _output_get_2 0)
          (set `self.MisionPapyrusCompleted` true)
          (bind _asthird_person_character (cast `/Game/ThirdPersonBP/Blueprints/ThirdPersonCharacter` (`GameplayStatics.GetPlayerCharacter` 0)))
          (`/Game/ThirdPersonBP/Blueprints/ThirdPersonCharacter.Isla Mision Completed` _asthird_person_character)
          (`MaterialInstanceDynamic.SetScalarParameterValue` (`self.MaterialDynamicIzq`) "Tallado" 1.0)
          (`MaterialInstanceDynamic.SetScalarParameterValue` (`self.MaterialDynamicDer`) "Tallado" 1.0))))))

(event `self.BoxChangeLevel.OnComponentBeginOverlap`
  (params (OverlappedComponent :type "PrimitiveComponent Object Reference") (OtherActor :type "Actor Object Reference") (OtherComp :type "PrimitiveComponent Object Reference") (OtherBodyIndex :type Integer) (bFromSweep :type Boolean) (SweepResult :type "HitResult Structure (by ref)"))
  (cast `/Game/ThirdPersonBP/Blueprints/ThirdPersonCharacter` OtherActor)
  (`GameplayStatics.OpenLevel` "Ruins"))

(event `self.InteractOpenDoors.OnComponentBeginOverlap`
  (params (OverlappedComponent :type "PrimitiveComponent Object Reference") (OtherActor :type "Actor Object Reference") (OtherComp :type "PrimitiveComponent Object Reference") (OtherBodyIndex :type Integer) (bFromSweep :type Boolean) (SweepResult :type "HitResult Structure (by ref)"))
  (if (and (`self.MisionRocksCompleted`) (`self.DoorsClosed`))
    (bind _asthird_person_character (cast `/Game/ThirdPersonBP/Blueprints/ThirdPersonCharacter` OtherActor))
    (add `/Game/ThirdPersonBP/Blueprints/ThirdPersonCharacter.InteractPressed` _asthird_person_character (delegate `CustomEvent_0`))
    (`/Game/ThirdPersonBP/Blueprints/ThirdPersonCharacter.ConstructInteractWidget` _asthird_person_character)))

(event `CustomEvent_0`
  (if (`self.DoorsClosed`)
    (set `self.LevelCompleted` true)
    (`self.OpenDoors`)
    (remove `/Game/ThirdPersonBP/Blueprints/ThirdPersonCharacter.InteractPressed` (stale `self.InteractOpenDoors.OnComponentBeginOverlap` _asthird_person_character) (delegate `CustomEvent_0`))
    (`/Game/ThirdPersonBP/Blueprints/ThirdPersonCharacter.DestroyInteractionWidget` (stale `self.InteractOpenDoors.OnComponentBeginOverlap` _asthird_person_character))
    (`/Game/ThirdPersonBP/Blueprints/ThirdPersonCharacter.Isla Level Completed` (stale `self.InteractOpenDoors.OnComponentBeginOverlap` _asthird_person_character))))

(event `self.InteractOpenDoors.OnComponentEndOverlap`
  (params (OverlappedComponent :type "PrimitiveComponent Object Reference") (OtherActor :type "Actor Object Reference") (OtherComp :type "PrimitiveComponent Object Reference") (OtherBodyIndex :type Integer))
  (bind _asthird_person_character (cast `/Game/ThirdPersonBP/Blueprints/ThirdPersonCharacter` OtherActor))
  (remove `/Game/ThirdPersonBP/Blueprints/ThirdPersonCharacter.InteractPressed` _asthird_person_character (delegate `CustomEvent_0`))
  (`/Game/ThirdPersonBP/Blueprints/ThirdPersonCharacter.DestroyInteractionWidget` _asthird_person_character))

(event `OpenDoors`
  (bind (_direction _doorrotation) (`Timeline|DoorMovement`)
    (:`Update`
      (`SceneComponent.K2_SetRelativeRotation` (`self.Right`) (`KismetMathLibrary.RLerp` (struct) (struct :`Pitch` -95.0) _doorrotation true) false false)
      (`SceneComponent.K2_SetRelativeRotation` (`self.Left`) (`KismetMathLibrary.RLerp` (struct) (struct :`Pitch` 95.0) _doorrotation true) false false))
    (:`Finished`
      (set `self.DoorsClosed` false))))

(fn `UserConstructionScript`
  (`|ExecutionSequence`
    (:`then_0`
      (bind _returnvalue (`KismetMaterialLibrary.CreateDynamicMaterialInstance` "/Game/Isla/Prueba_Puzzle/Puerta/Bloques/Bloque_Der_CE.Bloque_Der_CE"))
      (bind _output_get (set `self.MaterialDynamicDer` _returnvalue))
      (`PrimitiveComponent.SetMaterial` (`self.Right`) 1 _output_get))
    (:`then_1`
      (bind _returnvalue_2 (`KismetMaterialLibrary.CreateDynamicMaterialInstance` "/Game/Isla/Prueba_Puzzle/Puerta/Bloques/Bloque_Izq_CE.Bloque_Izq_CE"))
      (bind _output_get_2 (set `self.MaterialDynamicIzq` _returnvalue_2))
      (`PrimitiveComponent.SetMaterial` (`self.Left`) 1 _output_get_2))))