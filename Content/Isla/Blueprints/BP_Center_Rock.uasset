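; BP_Center_Rock is a center rock actor that reacts to the player and highlights symbols on a surrounding BP_Border.
; ThirdPersonCharacter overlapping its capsule plays a timeline that moves the Center component's relative location, and leaving reverses it.
; Each tick, a visibility trace along its Arrow selects the hit BP_Border component when it changes.
; When the trace misses, it calls SetSelected with no component on the cached border.
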(event `self.Capsule.OnComponentBeginOverlap`
  (params (OverlappedComponent :type "PrimitiveComponent Object Reference") (OtherActor :type "Actor Object Reference") (OtherComp :type "PrimitiveComponent Object Reference") (OtherBodyIndex :type Integer) (bFromSweep :type Boolean) (SweepResult :type "HitResult Structure (by ref)"))
  ;[1 1 1] Rotation
  (cast `/Game/ThirdPersonBP/Blueprints/ThirdPersonCharacter` OtherActor)
  (bind (_direction _center_rock_track) (`Timeline|Rock Center TL` :!label _label)
    (:`Update`
      (`SceneComponent.K2_SetRelativeLocation` (`self.Center`) (`KismetMathLibrary.VLerp` _center_rock_track (0.0 0.0 -15.0)) false false))))

(event `self.Capsule.OnComponentEndOverlap`
  (params (OverlappedComponent :type "PrimitiveComponent Object Reference") (OtherActor :type "Actor Object Reference") (OtherComp :type "PrimitiveComponent Object Reference") (OtherBodyIndex :type Integer))
  ;[1 1 1] Rotation
  (cast `/Game/ThirdPersonBP/Blueprints/ThirdPersonCharacter` OtherActor)
  (goto _label :!via `Reverse`))

(event `self.ReceiveTick`
  (params (DeltaSeconds :type "Float (single-precision)"))
  (bind _arrow (`self.Arrow`))
  (bind _border_actor (`self.Border_Actor`))
  (bind _returnvalue (`SceneComponent.K2_GetComponentLocation` _arrow))
  ;[1 1 1] Symbols
  (bind _outhit (`KismetSystemLibrary.LineTraceSingle` _returnvalue (+ _returnvalue (* (`SceneComponent.GetForwardVector` _arrow) 1000.0)) "TraceTypeQuery1" true))
  (bind (_bblockinghit _binitialoverlap _time _distance _location _impactpoint _normal _impactnormal _physmat _hitactor _hitcomponent) (`GameplayStatics.BreakHitResult` _outhit))
  (bind _asbp_border (cast `/Game/Isla/Blueprints/BP_Border` _hitactor)
    (:`then`
      (`/Engine/EditorBlueprintResources/StandardMacros.IsValid` (`self.Border_Actor`)
        (:`Is Valid`
          _)
        (:`Is Not Valid`
          (set `self.Border_Actor` _asbp_border)))
      (if (!= _hitcomponent (`self.HitComponent`))
        (bind _output_get (set `self.HitComponent` _hitcomponent))
        (`/Game/Isla/Blueprints/BP_Border.SetSelected` _asbp_border _output_get)))
    (:`CastFailed`
      (`/Engine/EditorBlueprintResources/StandardMacros.IsValid` _border_actor
        (:`Is Valid`
          (`/Game/Isla/Blueprints/BP_Border.SetSelected` _border_actor null))))))

(fn `UserConstructionScript`)