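; BP_Column_Sensor is a column in the Ruinas laser puzzle that visually switches on and off through material swaps.
; ToggleState compares the requested state with the column's current material and ignores calls that match it.
; Turning on shows a power-up material, then an oscillating one after a delay.
; Turning off shows a power-down material, then the unlit ruins wall material after a delay.
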(event `/Game/Ruinas/PuzzleLasers/BPI_SetState.Toggle State`
  (params (`On/Off` :type Boolean))
  (bind _columna (`self.Columna`))
  (bind _returnvalue (`PrimitiveComponent.GetMaterial` (`self.Columna`) 0))
  (bind _output_get (set `self.On/Off` `On/Off`))
  (if (== _output_get (or (== _returnvalue "/Game/Ruinas/Materials/Columna/M_Columna_Prender.M_Columna_Prender") (== _returnvalue "/Game/Ruinas/Materials/Columna/M_Columna_Oscilar.M_Columna_Oscilar")))
    _
    (elif _output_get
      (`PrimitiveComponent.SetMaterialByName` _columna "Material #43" "/Game/Ruinas/Materials/Columna/M_Columna_Prender.M_Columna_Prender")
      (`KismetSystemLibrary.Delay` 2.0)
      (`PrimitiveComponent.SetMaterialByName` _columna "Material #43" "/Game/Ruinas/Materials/Columna/M_Columna_Oscilar.M_Columna_Oscilar")
      (else
        (`PrimitiveComponent.SetMaterialByName` _columna "Material #43" "/Game/Ruinas/Materials/Columna/M_Columna_Apagar.M_Columna_Apagar")
        (`KismetSystemLibrary.Delay` 1.5)
        (`PrimitiveComponent.SetMaterialByName` _columna "Material #43" "/Game/Ruinas/Materials/Columna/M_Ruins_Walls_Apagado.M_Ruins_Walls_Apagado")))))

(fn `UserConstructionScript`)