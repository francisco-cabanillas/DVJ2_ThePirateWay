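; BP_Laser is a laser puzzle beam that bounces off mirrors to switch on sensors.
; CastLight switches off the remembered sensor, then line traces in a loop, reflecting wherever the hit face's material is Mirror.
; Two other material matches send an on message to the hit actor, only the first storing it as the active sensor.
; Any non-mirror hit or miss ends the loop, and debug trace lines draw the path.
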(fn `CastLight`
  (params (CastOrigin :type "Vector Structure") (`Cast Direction` :type "Vector Structure") (`Cast Distance` :type "Float (double-precision)"))
  (locals (L_CastOrigin :type "Vector Structure") (L_CastDirection :type "Vector Structure") (L_CastDistance :type "Float (double-precision)") (ActivatedSensor :type "Actor Object Reference") (L_Continue :type Boolean :default true))
  (bind _l_castorigin (`local.L_CastOrigin`))
  (set `local.L_CastOrigin` CastOrigin)
  (set `local.L_CastDirection` `Cast Direction`)
  (set `local.L_CastDistance` `Cast Distance`)
  (message `/Game/Ruinas/PuzzleLasers/BPI_SetState.Toggle State` (`local.ActivatedSensor`) false)
  (while (`local.L_Continue`)
    (bind (_outhit _returnvalue) (`KismetSystemLibrary.LineTraceSingle` :`Start` _l_castorigin :`End` (+ _l_castorigin (* (`local.L_CastDirection`) (`local.L_CastDistance`))) :`TraceChannel` "TraceTypeQuery3" :`bTraceComplex` true :`DrawDebugType` "ForDuration" :`TraceColor` (struct :`R` 0.788641 :`B` 0.0348 :`A` 1.0) :`TraceHitColor` (`KismetMathLibrary.LinearColor_Transparent`) :`DrawTime` 0.1))
    (if _returnvalue
      (bind (_bblockinghit _binitialoverlap _time _distance _location _impactpoint _normal _impactnormal _physmat _hitactor _hitcomponent _hitbonename _hititem _elementindex _faceindex) (`GameplayStatics.BreakHitResult` _outhit))
      (bind (_sectionindex _returnvalue_2) (`PrimitiveComponent.GetMaterialFromCollisionFaceIndex` _hitcomponent _faceindex))
      (if (== _returnvalue_2 "/Game/Ruinas/PuzzleLasers/Mirror.Mirror")
        (set `local.L_CastOrigin` _impactpoint)
        (set `local.L_CastDirection` (`KismetMathLibrary.MirrorVectorByNormal` (`local.L_CastDirection`) _normal))
        (set `local.L_Continue` true)
        (else
          (if (== _returnvalue_2 null)
            (message `/Game/Ruinas/PuzzleLasers/BPI_SetState.Toggle State` _hitactor true)
            (set `local.ActivatedSensor` _hitactor)
            (elif (== _returnvalue_2 null)
              (message `/Game/Ruinas/PuzzleLasers/BPI_SetState.Toggle State` _hitactor true)))
          (set `local.L_Continue` false :!label _label)))
      (else
        (goto _label)))))

(fn `UserConstructionScript`)