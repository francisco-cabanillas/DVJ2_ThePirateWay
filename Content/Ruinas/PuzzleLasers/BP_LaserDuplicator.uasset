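; Laser puzzle piece, named as a duplicator, that re-emits an incoming beam from its own Sphere component.
; Reflection calls CastLight from the sphere's location with the received Distance, ignoring the hit Origin and Normal.
; The rotation offset is built from a zero vector, so the beam keeps its incoming direction.
; Only one cast is wired, so no second beam is produced here.
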(fn `Reflection`
  (params (Origin :type "Vector Structure") (Direction :type "Vector Structure") (Distance :type "Float (double-precision)") (Normal :type "Vector Structure"))
  (if true
    (`|ExecutionSequence`
      (:`then_0`
        (`self.CastLight` (`SceneComponent.K2_GetComponentLocation` (`self.Sphere`)) (`KismetMathLibrary.GetForwardVector` (`KismetMathLibrary.Conv_VectorToRotator` (`KismetMathLibrary.GreaterGreater_VectorRotator` Direction (`KismetMathLibrary.Conv_VectorToRotator` (0.0 0.0 0.0))))) Distance)))))

(fn `UserConstructionScript`)