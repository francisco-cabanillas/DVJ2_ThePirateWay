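; Laser emitter for the ruins puzzle that fires a mirror-bounced beam and checks for puzzle completion.
; Every Tick it clears all BP_Reflection flags, line-traces along its Arrow to set the Niagara beam, and calls Reflection on mirror-material hits.
; It also counts lit column sensors out of four, updates the GameMode and adds a new mission widget each pass.
; With none left, it latches solved, opens doors and ends the game.
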(event `self.ReceiveTick`
  (params (DeltaSeconds :type "Float (single-precision)"))
  (`self.IniciarRayo`))

(fn `IniciarRayo`
  (bind _castdistance (`self.CastDistance`))
  (bind _arrow (`self.Arrow`))
  (bind _laserbeam (`self.LaserBeam`))
  (bind _returnvalue (`SceneComponent.K2_GetComponentLocation` _arrow))
  (bind _returnvalue_2 (`SceneComponent.GetForwardVector` _arrow))
  (bind _outactors (`GameplayStatics.GetAllActorsOfClass` "/Game/Ruinas/PuzzleLasers/BP_Reflection.BP_Reflection_C"))
  (for _array_element _outactors
    (set `/Game/Ruinas/PuzzleLasers/BP_Reflection.Activo` false _array_element)
    (set `/Game/Ruinas/PuzzleLasers/BP_Reflection.Activo2` false _array_element))
  (if (not (`self.Decifrado`))
    (`|ExecutionSequence`
      (:`then_0`
        (bind _outhit (`KismetSystemLibrary.LineTraceSingle` :`Start` _returnvalue :`End` (+ _returnvalue (* _returnvalue_2 _castdistance)) :`TraceChannel` "TraceTypeQuery3" :`TraceHitColor` (struct)))
        (`FXSystemComponent.SetFloatParameter` _laserbeam "User.Beam Width" 5.0)
        (bind (_bblockinghit _binitialoverlap _time _distance _location _impactpoint _normal _impactnormal _physmat _hitactor _hitcomponent) (`GameplayStatics.BreakHitResult` _outhit))
        (`FXSystemComponent.SetVectorParameter` _laserbeam "User.Beam End" _location)
        (bind _asbp_mirror (cast `/Game/Ruinas/PuzzleLasers/BP_Mirror` _hitactor))
        (bind (_sectionindex _returnvalue_3) (`PrimitiveComponent.GetMaterialFromCollisionFaceIndex` _hitcomponent 0))
        (if (or (== _returnvalue_3 "/Game/Ruinas/espejo3/M_espejo.M_espejo") (== _returnvalue_3 "/Game/Ruinas/espejo1/M_espejo1_3.M_espejo1_3"))
          (`/Game/Ruinas/PuzzleLasers/BP_Reflection.Reflection` _asbp_mirror _impactpoint _returnvalue_2 _castdistance _normal 0)))
      (:`then_1`
        (bind _outactors_2 (`GameplayStatics.GetAllActorsOfClass` "/Game/Ruinas/PuzzleLasers/BP_Column_Sensor.BP_Column_Sensor_C"))
        (set `self.CantDecifrados` 0)
        (for _array_element_2 _outactors_2
          (if (`/Game/Ruinas/PuzzleLasers/BP_Column_Sensor.On/Off` _array_element_2)
            (`/Engine/EditorBlueprintResources/StandardMacros.IncrementInt` (`self.CantDecifrados`))))
        (bind _asthird_person_game_mode (cast `/Game/ThirdPersonBP/Blueprints/ThirdPersonGameMode` (`GameplayStatics.GetGameMode`)))
        (set `/Game/ThirdPersonBP/Blueprints/ThirdPersonGameMode.ColumnSensorsLeft` (- 4 (`self.CantDecifrados`)) _asthird_person_game_mode)
        (bind _returnvalue_4 (`|CreateWidget` "/Game/InGameOverlay/Misions/LaserMisionWidget.LaserMisionWidget_C"))
        (`UserWidget.AddToViewport` _returnvalue_4 0)
        (bind _asthird_person_game_mode_2 (cast `/Game/ThirdPersonBP/Blueprints/ThirdPersonGameMode` (`GameplayStatics.GetGameMode`)))
        (if (== (`/Game/ThirdPersonBP/Blueprints/ThirdPersonGameMode.ColumnSensorsLeft` _asthird_person_game_mode_2) 0)
          (set `self.Decifrado` true)
          (bind _asthird_person_character (cast `/Game/ThirdPersonBP/Blueprints/ThirdPersonCharacter` (`GameplayStatics.GetPlayerCharacter` 0)))
          (`/Game/ThirdPersonBP/Blueprints/ThirdPersonCharacter.Slide Off` _asthird_person_character)
          (bind _outactors_3 (`GameplayStatics.GetAllActorsOfClass` "/Game/Ruinas/PuzzleLasers/BP_Door.BP_Door_C"))
          (`/Game/Ruinas/PuzzleLasers/Door_Interface.Open door` _outactors_3)
          (`GameplayStatics.PlaySound2D` "/Game/StarterContent/Audio/misionCompleted.misionCompleted" 1.0 1.0 0.0 null null)
          (`/Game/ThirdPersonBP/Blueprints/ThirdPersonCharacter.DestroyLeftRightWidget` _asthird_person_character)
          (`/Game/ThirdPersonBP/Blueprints/ThirdPersonCharacter.EndGame` _asthird_person_character))))))

(fn `UserConstructionScript`)