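; BP_Mirror is a laser puzzle mirror that reflects light and that the player can rotate.
; While a ThirdPersonCharacter overlaps its Box, it binds to that character's left/right input and has it show a left/right widget.
; Each press sets actor yaw 22.5 degrees either way from BPReflection's relative rotation.
; Reflection mirrors the incoming direction about the surface normal and passes it to CastLight.
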(event `self.Box.OnComponentBeginOverlap`
  (params (OverlappedComponent :type "PrimitiveComponent Object Reference") (OtherActor :type "Actor Object Reference") (OtherComp :type "PrimitiveComponent Object Reference") (OtherBodyIndex :type Integer) (bFromSweep :type Boolean) (SweepResult :type "HitResult Structure (by ref)"))
  (bind _asthird_person_character (cast `/Game/ThirdPersonBP/Blueprints/ThirdPersonCharacter` OtherActor))
  (add `/Game/ThirdPersonBP/Blueprints/ThirdPersonCharacter.LeftRightPressed` _asthird_person_character (delegate `CustomEvent_0`))
  (`/Game/ThirdPersonBP/Blueprints/ThirdPersonCharacter.ConstructLeftRightWidget` _asthird_person_character))

(event `CustomEvent_0`
  (params (Q :type Boolean))
  (bind _returnvalue (`SceneComponent.GetRelativeTransform` (`self.BP_Reflection`)))
  (bind _returnvalue_2 (`SceneComponent.GetRelativeTransform` (`self.BP_Reflection`)))
  (if Q
    (`self.K2_SetActorRelativeRotation` (`KismetMathLibrary.MakeRotator` (.roll (.rotation _returnvalue)) (.pitch (.rotation _returnvalue)) (+ (.yaw (.rotation _returnvalue)) 22.5)))
    (else
      (`self.K2_SetActorRotation` (`KismetMathLibrary.MakeRotator` (.roll (.rotation _returnvalue_2)) (.pitch (.rotation _returnvalue_2)) (+ (.yaw (.rotation _returnvalue_2)) -22.5))))))

(event `self.Box.OnComponentEndOverlap`
  (params (OverlappedComponent :type "PrimitiveComponent Object Reference") (OtherActor :type "Actor Object Reference") (OtherComp :type "PrimitiveComponent Object Reference") (OtherBodyIndex :type Integer))
  (bind _asthird_person_character (cast `/Game/ThirdPersonBP/Blueprints/ThirdPersonCharacter` OtherActor))
  (remove `/Game/ThirdPersonBP/Blueprints/ThirdPersonCharacter.LeftRightPressed` _asthird_person_character (delegate `CustomEvent_0`))
  (`/Game/ThirdPersonBP/Blueprints/ThirdPersonCharacter.DestroyLeftRightWidget` _asthird_person_character))

(fn `Reflection`
  (params (Origin :type "Vector Structure") (Direction :type "Vector Structure") (Distance :type "Float (double-precision)") (Normal :type "Vector Structure"))
  (`self.CastLight` Origin (`KismetMathLibrary.MirrorVectorByNormal` Direction Normal) Distance))

(fn `UserConstructionScript`)