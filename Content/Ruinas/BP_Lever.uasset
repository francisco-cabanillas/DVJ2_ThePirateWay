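; BP_Lever is a ruins lever that resets the rising sand and also starts and ends the ruins mission.
; Its trigger offers an interact prompt when a BP_Reaching_Sand passes height and direction checks, and removes it on leaving.
; LowerSand animates the lever and resets the first sand actor found, or plays a jammed sound if already animating.
; Start and Exit volumes toggle the mission on the character, with Exit also calling LowerSand.
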(event `self.TriggerPalanca.OnComponentBeginOverlap`
  (params (OverlappedComponent :type "PrimitiveComponent Object Reference") (OtherActor :type "Actor Object Reference") (OtherComp :type "PrimitiveComponent Object Reference") (OtherBodyIndex :type Integer) (bFromSweep :type Boolean) (SweepResult :type "HitResult Structure (by ref)"))
  ;[1 1 1] Lower Sand
  (bind _outactors (`GameplayStatics.GetAllActorsOfClass` "/Game/Ruinas/BP_Reaching_Sand.BP_Reaching_Sand_C"))
  (for _array_element _outactors
    (bind (_returnvalue_x _returnvalue_y _returnvalue_z) (`KismetMathLibrary.BreakVector` (`SceneComponent.K2_GetComponentLocation` (`/Game/Ruinas/BP_Reaching_Sand.Arena_No_Mover` _array_element))))
    (if (and (> _returnvalue_z -600.0) (>= (`/Game/Ruinas/BP_Reaching_Sand.move_direction` _array_element) 0.0))
      (`|ExecutionSequence`
        (:`then_0`
          (bind _asthird_person_character (cast `/Game/ThirdPersonBP/Blueprints/ThirdPersonCharacter` OtherActor))
          (add `/Game/ThirdPersonBP/Blueprints/ThirdPersonCharacter.InteractPressed` _asthird_person_character (delegate `LowerSand`))
          (`/Game/ThirdPersonBP/Blueprints/ThirdPersonCharacter.ConstructInteractWidget` _asthird_person_character))
        (:`then_1`
          (break))))))

(event `LowerSand`
  (bind _palanca1 (`self.palanca1`))
  ;[1 1 1] Lower Sand
  (if (`SkeletalMeshComponent.IsPlaying` (`self.palanca1`))
    (`GameplayStatics.SpawnSoundAttached` "/Game/Audio/Ruinas/Palanca/fx_palanca_ruinas_trancada_Cue.fx_palanca_ruinas_trancada_Cue" _palanca1 "None" (0.0 0.0 0.0) (struct) "KeepRelativeOffset" false 1.0 1.0 0.0 null null)
    (else
      (`SkeletalMeshComponent.PlayAnimation` _palanca1 "/Game/Ruinas/Palanca/palanca_Anim.palanca_Anim" false)
      (`GameplayStatics.SpawnSoundAttached` "/Game/Audio/Ruinas/Palanca/fx_palanca_ruinas_Cue.fx_palanca_ruinas_Cue" _palanca1 "None" (0.0 0.0 0.0) (struct) "KeepRelativeOffset" false 1.0 1.0 0.0 null null)
      (bind _outactors (`GameplayStatics.GetAllActorsOfClass` "/Game/Ruinas/BP_Reaching_Sand.BP_Reaching_Sand_C"))
      (for _array_element _outactors
        (`/Game/Ruinas/BP_Reaching_Sand.Reset Sand` _array_element)
        (break))
      (remove `/Game/ThirdPersonBP/Blueprints/ThirdPersonCharacter.InteractPressed` (stale `self.TriggerPalanca.OnComponentEndOverlap` _asthird_person_character) (delegate `LowerSand`) :!label _label)
      (`/Game/ThirdPersonBP/Blueprints/ThirdPersonCharacter.DestroyInteractionWidget` (stale `self.TriggerPalanca.OnComponentEndOverlap` _asthird_person_character)))))

(event `self.TriggerPalanca.OnComponentEndOverlap`
  (params (OverlappedComponent :type "PrimitiveComponent Object Reference") (OtherActor :type "Actor Object Reference") (OtherComp :type "PrimitiveComponent Object Reference") (OtherBodyIndex :type Integer))
  ;[1 1 1] Lower Sand
  (bind _asthird_person_character (cast `/Game/ThirdPersonBP/Blueprints/ThirdPersonCharacter` OtherActor))
  (goto _label))

(event `self.Start.OnComponentEndOverlap`
  (params (OverlappedComponent :type "PrimitiveComponent Object Reference") (OtherActor :type "Actor Object Reference") (OtherComp :type "PrimitiveComponent Object Reference") (OtherBodyIndex :type Integer))
  ;[1 1 1] Start Mision
  (bind _asthird_person_character (cast `/Game/ThirdPersonBP/Blueprints/ThirdPersonCharacter` OtherActor))
  (if (not (`self.Mision`))
    (set `self.Mision` true)
    (`/Game/ThirdPersonBP/Blueprints/ThirdPersonCharacter.StartMisionRuina` _asthird_person_character)))

(event `self.Exit.OnComponentEndOverlap`
  (params (OverlappedComponent :type "PrimitiveComponent Object Reference") (OtherActor :type "Actor Object Reference") (OtherComp :type "PrimitiveComponent Object Reference") (OtherBodyIndex :type Integer))
  ;[1 1 1] Start Mision
  (bind _asthird_person_character (cast `/Game/ThirdPersonBP/Blueprints/ThirdPersonCharacter` OtherActor))
  (if (`self.Mision`)
    (set `self.Mision` false)
    (`/Game/ThirdPersonBP/Blueprints/ThirdPersonCharacter.EndMisionRuina` _asthird_person_character)
    (`self.LowerSand`)))

(fn `UserConstructionScript`)