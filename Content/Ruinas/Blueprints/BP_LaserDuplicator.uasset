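; BP_LaserDuplicator is a beam-splitter for a laser puzzle, turning an incoming ray into two outgoing ones.
; Reflection increments the caller's ray ID, then calls CastLight twice from the Sphere's location, passing the incoming distance.
; The two directions point left and right, perpendicular to the incoming direction; the hit normal is unused.
; A FirstTurnOn flag limits the splitter sound to the first activation.
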(fn `Reflection`
  (params (Origin :type "Vector Structure") (Direction :type "Vector Structure") (Distance :type "Float (double-precision)") (Normal :type "Vector Structure") (Id_Rayo_caller :type Integer))
  (bind _returnvalue (`KismetMathLibrary.Conv_VectorToRotator` Direction))
  (bind _sphere (`self.Sphere`))
  (if (`self.first_turn_on`)
    (`GameplayStatics.PlaySoundAtLocation` "/Game/Audio/Ruinas/Espejos/fx_divisor_Cue.fx_divisor_Cue" Origin (struct) 1.0 1.0 0.0 null null null)
    (set `self.first_turn_on` false))
  (set `self.Id_Rayo` (+ Id_Rayo_caller 1))
  (`|ExecutionSequence`
    (:`then_0`
      (`self.CastLight` (`SceneComponent.K2_GetComponentLocation` _sphere) (`KismetMathLibrary.GetForwardVector` (`KismetMathLibrary.Conv_VectorToRotator` (`KismetMathLibrary.GreaterGreater_VectorRotator` (0.0 -90.0 0.0) _returnvalue))) Distance))
    (:`then_1`
      (`self.CastLight` (`SceneComponent.K2_GetComponentLocation` _sphere) (`KismetMathLibrary.GetForwardVector` (`KismetMathLibrary.Conv_VectorToRotator` (`KismetMathLibrary.GreaterGreater_VectorRotator` (0.0 90.0 0.0) _returnvalue))) Distance))))

(fn `UserConstructionScript`)