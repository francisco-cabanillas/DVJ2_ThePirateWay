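; Rising-sand hazard for the Ruinas level that moves ArenaMover between bottom and top heights as a timed challenge.
; A character entering the Box starts the slow rise, seeks the music to match progress, and drives that player's Timer from Tick.
; Reaching the top triggers the player's lower-sand mission.
; ResetSand stops the music, lowers the sand faster, ends that mission and resets every BP_Mirror rotation.
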(event `Reset Sand`
  (bind _timer (`self.Timer`))
  (bind _top_height (`self.top_height`))
  (bind (_returnvalue_x _returnvalue_y _returnvalue_z) (`KismetMathLibrary.BreakVector` (`SceneComponent.K2_GetComponentLocation` (`self.Arena_Mover`))))
  (bind _z (.z (`SceneComponent.K2_GetComponentLocation` (`self.Arena_Mover`))))
  (bind _returnvalue (> _z (`self.top_height`)))
  (`AudioComponent.Stop` (`self.Music_ruinas`))
  (if (>= _returnvalue_z _top_height)
    (`SceneComponent.K2_SetWorldLocation` (`self.Arena_Mover`) (`KismetMathLibrary.MakeVector` _returnvalue_x _returnvalue_y (+ _top_height -1.0)) false false))
  (bind _output_get (set `self.move_direction` -3.0))
  (set `self.progress_bar_change` (/ (* _output_get 100.0) (- (`self.bottom_height`) (`self.top_height`))))
  (set `self.sand_moving` true)
  (`/Game/Personaje/Blueprints/ThirdPersonCharacter.EndMissionLowerSand` (`self.player`))
  (bind _outactors (`GameplayStatics.GetAllActorsOfClass` "/Game/Ruinas/Blueprints/BP_Mirror.BP_Mirror_C"))
  (for _array_element _outactors
    (`/Game/Ruinas/Blueprints/BP_Mirror.ResetRotation` _array_element)
    (bind _output_get_2 (set `self.Current_Porcentage` (+ (`self.Current_Porcentage`) (* (stale `self.ReceiveTick` DeltaSeconds) (`self.progress_bar_change`))) :!label _label))
    (`/Engine/EditorBlueprintResources/StandardMacros.IsValid` _timer
      (:`Is Valid`
        (`/Game/UI/Misions/HUD_Timer.Move_Timer` _timer _output_get_2)
        (`SceneComponent.K2_SetWorldLocation` (`self.Arena_Mover`) (`KismetMathLibrary.MakeVector` (.x (`SceneComponent.K2_GetComponentLocation` (`self.Arena_Mover`))) (.y (`SceneComponent.K2_GetComponentLocation` (`self.Arena_Mover`))) (+ _z (* (stale `self.ReceiveTick` DeltaSeconds) (`self.move_direction`)))) false false)
        (if (or _returnvalue (< _z (`self.bottom_height`)))
          (set `self.sand_moving` false)
          (set `self.move_direction` 0.0)
          (if _returnvalue
            (`/Game/Personaje/Blueprints/ThirdPersonCharacter.StartMissionLowerSand` (`self.player`))))))))

(event `self.ReceiveTick`
  (params (DeltaSeconds :type "Float (single-precision)"))
  (if (`self.sand_moving`)
    (goto _label)))

(event `self.Box.OnComponentBeginOverlap`
  (params (OverlappedComponent :type "PrimitiveComponent Object Reference") (OtherActor :type "Actor Object Reference") (OtherComp :type "PrimitiveComponent Object Reference") (OtherBodyIndex :type Integer) (bFromSweep :type Boolean) (SweepResult :type "HitResult Structure (by ref)"))
  (bind _move_direction (`self.move_direction`))
  (bind _bottom_height (`self.bottom_height`))
  (bind _sand_moving (`self.sand_moving`))
  (bind (_returnvalue_x _returnvalue_y _returnvalue_z) (`KismetMathLibrary.BreakVector` (`SceneComponent.K2_GetComponentLocation` (`self.Arena_Mover`))))
  (if (or (and (not _sand_moving) (== _move_direction 0.0)) (and _sand_moving (< _move_direction 0.0)))
    (bind _asthird_person_character (cast `/Game/Personaje/Blueprints/ThirdPersonCharacter` OtherActor))
    (set `self.player` _asthird_person_character)
    (if (>= _bottom_height _returnvalue_z)
      (`SceneComponent.K2_SetWorldLocation` (`self.Arena_Mover`) (`KismetMathLibrary.MakeVector` _returnvalue_x _returnvalue_y (+ _bottom_height 1.0)) false false))
    (set `self.sand_moving` true)
    (`AudioComponent.Play` (`self.Music_ruinas`) (/ (* 300.0 (`KismetMathLibrary.Abs` (- (`self.Current_Porcentage`) 100.0))) 100.0))
    (bind _output_get (set `self.move_direction` 0.8))
    (set `self.Timer` (`/Game/Personaje/Blueprints/ThirdPersonCharacter.Timer` _asthird_person_character))
    (set `self.progress_bar_change` (/ (* _output_get 100.0) (- (`self.bottom_height`) (`self.top_height`))))
    (goto _label)))

(fn `UserConstructionScript`)