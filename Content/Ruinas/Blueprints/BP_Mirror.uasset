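; BP_Mirror is a rotatable mirror that redirects light beams from BP_LaserEmitter.
; While the ThirdPersonCharacter overlaps its box, it shows a left/right widget and binds input that snaps yaw 45 degrees, plays a sound and restarts the emitter's ray.
; Reflection increments the ray ID when inactive and casts light along the normal-mirrored direction, keeping the original when axis magnitudes match.
; ResetRotation restores the starting rotation; a separate MoveMirror timeline interpolates rotation with debug prints.
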(event `MoveMirror`
  (params (Right :type Boolean))
  (bind _returnvalue (`SceneComponent.GetRelativeTransform` (`self.BP_Reflection`)))
  (bind (_direction _mirrormovement) (`Timeline|MirrorMovement` :!via `PlayFromStart`)
    (:`Update`
      (bind _returnvalue_2 (`KismetMathLibrary.MakeRotator` (.roll (.rotation _returnvalue)) (.pitch (.rotation _returnvalue)) (+ (.yaw (.rotation _returnvalue)) (`KismetMathLibrary.SelectFloat` 45.0 -45.0 (stale `CustomEvent_0` Q)))))
      (`self.K2_SetActorRotation` (`KismetMathLibrary.RLerp` (struct) _returnvalue_2 _mirrormovement true)))
    (:`Finished`
      (`KismetSystemLibrary.PrintString` "Hello")
      (`KismetSystemLibrary.PrintString` (`KismetStringLibrary.Conv_RotatorToString` _returnvalue_2)))))

(event `self.ReceiveBeginPlay`
  (bind (_returnvalue_location _returnvalue_rotation) (`KismetMathLibrary.BreakTransform` (`SceneComponent.GetRelativeTransform` (`self.BP_Reflection`))))
  (set `self.InitialRotation` _returnvalue_rotation))

(event `ResetRotation`
  (`self.K2_SetActorRotation` (`self.InitialRotation`))
  (bind _returnvalue (`GameplayStatics.GetActorOfClass` "/Game/Ruinas/Blueprints/BP_LaserEmitter.BP_LaserEmitter_C"))
  (`/Game/Ruinas/Blueprints/BP_LaserEmitter.IniciarRayo` _returnvalue))

(event `self.Box.OnComponentBeginOverlap`
  (params (OverlappedComponent :type "PrimitiveComponent Object Reference") (OtherActor :type "Actor Object Reference") (OtherComp :type "PrimitiveComponent Object Reference") (OtherBodyIndex :type Integer) (bFromSweep :type Boolean) (SweepResult :type "HitResult Structure (by ref)"))
  (bind _asthird_person_character (cast `/Game/Personaje/Blueprints/ThirdPersonCharacter` OtherActor))
  (add `/Game/Personaje/Blueprints/ThirdPersonCharacter.LeftRightPressed` _asthird_person_character (delegate `CustomEvent_0`))
  (`/Game/Personaje/Blueprints/ThirdPersonCharacter.ConstructLeftRightWidget` _asthird_person_character))

(event `CustomEvent_0`
  (params (Q :type Boolean))
  (bind _returnvalue (`SceneComponent.GetRelativeTransform` (`self.BP_Reflection`)))
  (`self.K2_SetActorRotation` (`KismetMathLibrary.MakeRotator` (.roll (.rotation _returnvalue)) (.pitch (.rotation _returnvalue)) (+ (.yaw (.rotation _returnvalue)) (`KismetMathLibrary.SelectFloat` 45.0 -45.0 Q))))
  (`GameplayStatics.PlaySoundAtLocation` "/Game/Audio/Ruinas/Espejos/fx_movimientoespejos_wet_Cue.fx_movimientoespejos_wet_Cue" (`SceneComponent.K2_GetComponentLocation` (`self.BP_Reflection`)) (struct) 1.0 1.0 0.0 null null null)
  (bind _returnvalue_2 (`GameplayStatics.GetActorOfClass` "/Game/Ruinas/Blueprints/BP_LaserEmitter.BP_LaserEmitter_C"))
  (`/Game/Ruinas/Blueprints/BP_LaserEmitter.IniciarRayo` _returnvalue_2))

(event `self.Box.OnComponentEndOverlap`
  (params (OverlappedComponent :type "PrimitiveComponent Object Reference") (OtherActor :type "Actor Object Reference") (OtherComp :type "PrimitiveComponent Object Reference") (OtherBodyIndex :type Integer))
  (bind _asthird_person_character (cast `/Game/Personaje/Blueprints/ThirdPersonCharacter` OtherActor))
  (remove `/Game/Personaje/Blueprints/ThirdPersonCharacter.LeftRightPressed` _asthird_person_character (delegate `CustomEvent_0`))
  (`/Game/Personaje/Blueprints/ThirdPersonCharacter.DestroyLeftRightWidget` _asthird_person_character))

(fn `Reflection`
  (params (Origin :type "Vector Structure") (Direction :type "Vector Structure") (Distance :type "Float (double-precision)") (Normal :type "Vector Structure") (Id_Rayo_caller :type Integer))
  (bind _returnvalue (`KismetMathLibrary.MirrorVectorByNormal` Direction Normal))
  (if (not (`self.Activo`))
    (set `self.Id_Rayo` (+ Id_Rayo_caller 1)))
  (if (== (- (`KismetMathLibrary.Vector_GetAbs` _returnvalue) (`KismetMathLibrary.Vector_GetAbs` Direction)) (0.0 0.0 0.0) :`ErrorTolerance` 0.1)
    (`self.CastLight` Origin Direction Distance)
    (else
      (`self.CastLight` Origin _returnvalue Distance))))

(fn `UserConstructionScript`)