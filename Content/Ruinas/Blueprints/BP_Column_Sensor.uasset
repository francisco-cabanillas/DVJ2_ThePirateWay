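; BP_Column_Sensor is a column that switches between on and off states with matching sound and material effects.
; The construction script gives the column mesh a dynamic M_Columna material instance.
; ToggleState skips repeated on requests through a NAND check, then plays a one-shot cue and drives the Switch and Oscilar parameters in delayed sequences.
; A looping sound starts after the switch-on delay and stops immediately on switch-off.
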(event `/Game/Ruinas/Blueprints/BPI_SetState.Toggle State`
  (params (`Trigger On/Off` :type Boolean))
  (bind _materialdynamiccolumn (`self.MaterialDynamicColumn`))
  (bind _audioloop (`self.AudioLoop`))
  (bind _returnvalue (`SceneComponent.K2_GetComponentLocation` (`self.Columna`)))
  (if (`KismetMathLibrary.BooleanNAND` `Trigger On/Off` (`self.IsOn`))
    (bind _output_get (set `self.IsOn` `Trigger On/Off`))
    (if _output_get
      (`GameplayStatics.PlaySoundAtLocation` "/Game/Audio/Ruinas/Columnas/fx_columna_on_Cue.fx_columna_on_Cue" _returnvalue (struct) 1.0 1.0 0.0 null null null)
      (`MaterialInstanceDynamic.SetScalarParameterValue` _materialdynamiccolumn "Switch" 1.0)
      (`KismetSystemLibrary.Delay` 1.8)
      (`MaterialInstanceDynamic.SetScalarParameterValue` _materialdynamiccolumn "Oscilar" 1.0)
      (`AudioComponent.Play` _audioloop 0.0)
      (`MaterialInstanceDynamic.SetScalarParameterValue` _materialdynamiccolumn "Switch" -1.0)
      (else
        (`AudioComponent.Stop` _audioloop)
        (`GameplayStatics.PlaySoundAtLocation` "/Game/Audio/Ruinas/Columnas/fx_columna_off_Cue.fx_columna_off_Cue" _returnvalue (struct) 1.0 1.0 0.0 null null null)
        (`MaterialInstanceDynamic.SetScalarParameterValue` _materialdynamiccolumn "Oscilar" 0.0)
        (`KismetSystemLibrary.Delay` 1.2)
        (`MaterialInstanceDynamic.SetScalarParameterValue` _materialdynamiccolumn "Switch" 0.0)))))

(fn `UserConstructionScript`
  (bind _returnvalue (`KismetMaterialLibrary.CreateDynamicMaterialInstance` "/Game/Ruinas/Materials/Columna/M_Columna.M_Columna"))
  (bind _output_get (set `self.MaterialDynamicColumn` _returnvalue))
  (`PrimitiveComponent.SetMaterial` (`self.Columna`) 0 _output_get))