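; BP_Reflection is the base actor for laser-reflecting puzzle pieces, passing light between mirrors and into column sensors.
; CastLight line-traces a Niagara-style beam, using hit materials to chain into the next piece's empty Reflection hook or switch on a sensor.
; BP_LaserDuplicator gets a second beam and target slot.
; Verificaciones detects changed targets; Desarmar recursively tears down downstream beams, using ray IDs to guard against loops.
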(fn `CastLight`
  (params (Origin :type "Vector Structure") (Direction :type "Vector Structure") (Distance :type "Float (double-precision)"))
  (bind _laserbeam (`self.LaserBeam`))
  (bind _laserbeam2 (`self.LaserBeam2`))
  (bind _outhit (`KismetSystemLibrary.LineTraceSingle` :`Start` Origin :`End` (+ Origin (* Direction Distance)) :`TraceChannel` "TraceTypeQuery3" :`bTraceComplex` true :`TraceHitColor` (struct)))
  (if (and (`self.Activo`) (== (`GameplayStatics.GetObjectClass` self) "/Game/Ruinas/Blueprints/BP_LaserDuplicator.BP_LaserDuplicator_C"))
    (`SceneComponent.K2_SetWorldLocation` _laserbeam2 Origin false false)
    (`FXSystemComponent.SetFloatParameter` _laserbeam2 "User.Beam Width" 5.0)
    (bind (_bblockinghit _binitialoverlap _time _distance _location _impactpoint _normal _impactnormal _physmat _hitactor _hitcomponent) (`GameplayStatics.BreakHitResult` _outhit))
    (`FXSystemComponent.SetVectorParameter` _laserbeam2 "User.Beam End" _impactpoint)
    (set `self.Activo2` true)
    (bind _resetactor (`self.Verificaciones` _hitactor (`self.Actor2`) _hitcomponent))
    (if _resetactor
      (set `self.Actor2` null))
    (else
      (`SceneComponent.K2_SetWorldLocation` _laserbeam Origin false false)
      (`FXSystemComponent.SetFloatParameter` _laserbeam "User.Beam Width" 5.0)
      (`FXSystemComponent.SetVectorParameter` _laserbeam "User.Beam End" _impactpoint)
      (set `self.Activo` true)
      (bind _resetactor_2 (`self.Verificaciones` _hitactor (`self.Actor`) _hitcomponent))
      (if _resetactor_2
        (set `self.Actor` null))))
  (bind (_sectionindex _returnvalue) (`PrimitiveComponent.GetMaterialFromCollisionFaceIndex` _hitcomponent 0))
  (if (and (!= _hitactor self) (or (== _returnvalue "/Game/Ruinas/Assets/espejo3/M_espejo.M_espejo") (== _returnvalue "/Game/Ruinas/Assets/espejo1/M_espejo1_3.M_espejo1_3") (== _returnvalue "/Game/Ruinas/Assets/espejo3/M_espejo3_4.M_espejo3_4")))
    (bind _asbp_reflection (cast `/Game/Ruinas/Blueprints/BP_Reflection` _hitactor))
    (bind _id_rayo (`/Game/Ruinas/Blueprints/BP_Reflection.Id_Rayo` _asbp_reflection))
    (if (or (== _id_rayo 0) (== _id_rayo (+ (`self.Id_Rayo`) 1)))
      (if (`self.Activo2`)
        (set `self.Actor2` _asbp_reflection)
        (else
          (set `self.Actor` _asbp_reflection)))
      (`self.Reflection` _asbp_reflection _impactpoint Direction Distance _normal (`self.Id_Rayo`)))
    (elif (or (== _returnvalue "/Game/Ruinas/Materials/Columna_Luz_Sensor/M_emissive.M_emissive") (== _returnvalue "/Game/Ruinas/Materials/Columna_Luz_Sensor/M_Columna_Luz_Sensor.M_Columna_Luz_Sensor"))
      (bind _asbp_column_sensor (cast `/Game/Ruinas/Blueprints/BP_Column_Sensor` _hitactor))
      (if (`self.Activo2`)
        (set `self.Actor2` _asbp_column_sensor)
        (else
          (set `self.Actor` _asbp_column_sensor)))
      (if (not (`/Game/Ruinas/Blueprints/BP_Column_Sensor.IsOn` _asbp_column_sensor))
        (`/Game/Ruinas/Blueprints/BP_Column_Sensor.Toggle State` _asbp_column_sensor true)))))

(fn `DeleteLaser`
  (bind _actor (`self.Actor`))
  (bind _actor2 (`self.Actor2`))
  (if (or (`self.Activo`) (`self.Activo2`))
    (if true
      (if (`self.Activo2`)
        (set `self.Activo` false)
        (set `self.Activo2` false)
        (bind _asbp_reflection (cast `/Game/Ruinas/Blueprints/BP_Reflection` _actor2)
          (:`then`
            (`self.DeleteLaser` _asbp_reflection))
          (:`CastFailed`
            _))
        (bind _asbp_column_sensor (cast `/Game/Ruinas/Blueprints/BP_Column_Sensor` _actor2)
          (:`then`
            (`/Game/Ruinas/Blueprints/BPI_SetState.Toggle State` _asbp_column_sensor false))
          (:`CastFailed`
            _))
        (else
          (set `self.Activo` false)
          (bind _asbp_reflection_2 (cast `/Game/Ruinas/Blueprints/BP_Reflection` _actor)
            (:`then`
              (`self.DeleteLaser` _asbp_reflection_2))
            (:`CastFailed`
              _))))
      (bind _asbp_column_sensor_2 (cast `/Game/Ruinas/Blueprints/BP_Column_Sensor` _actor))
      (`/Game/Ruinas/Blueprints/BPI_SetState.Toggle State` _asbp_column_sensor_2 false))))

(fn `Desarmar`
  (params (Id_caller :type Integer))
  (bind _actor2 (`self.Actor2`))
  (bind _actor (`self.Actor`))
  (bind _aux (`self.aux`))
  (bind _returnvalue (<= Id_caller (`self.aux`)))
  (set `self.first_turn_on` true)
  (set `self.aux` (`self.Id_Rayo`))
  (set `self.Id_Rayo` 0)
  (`|ExecutionSequence`
    (:`then_0`
      (bind _asbp_column_sensor (cast `/Game/Ruinas/Blueprints/BP_Column_Sensor` _actor2))
      (`/Game/Ruinas/Blueprints/BPI_SetState.Toggle State` _asbp_column_sensor false)
      (set `self.Actor2` null :!label _label)
      (set `self.Activo2` false))
    (:`then_1`
      (bind _asbp_column_sensor_2 (cast `/Game/Ruinas/Blueprints/BP_Column_Sensor` _actor))
      (`/Game/Ruinas/Blueprints/BP_Column_Sensor.Toggle State` _asbp_column_sensor_2 false)
      (set `self.Actor` null :!label _label_2)
      (set `self.Activo` false))
    (:`then_2`
      (`FXSystemComponent.SetFloatParameter` (`self.LaserBeam2`) "User.Beam Width" 0.0)
      (bind _asbp_reflection (cast `/Game/Ruinas/Blueprints/BP_Reflection` _actor2))
      (if _returnvalue
        (`self.Desarmar` _asbp_reflection _aux)
        (goto _label)))
    (:`then_3`
      (`FXSystemComponent.SetFloatParameter` (`self.LaserBeam`) "User.Beam Width" 0.0)
      (bind _asbp_reflection_2 (cast `/Game/Ruinas/Blueprints/BP_Reflection` _actor))
      (if _returnvalue
        (`self.Desarmar` _asbp_reflection_2 _aux)
        (goto _label_2)))))

(fn `Reflection`
  (params (Origin :type "Vector Structure") (Direction :type "Vector Structure") (Distance :type "Float (double-precision)") (Normal :type "Vector Structure") (Id_Rayo_caller :type Integer)))

(fn `UserConstructionScript`)

(fn `Verificaciones`
  (params (`Hit Actor` :type "Object Object Reference") (ActorInMemory :type "Actor Object Reference") (`Hit Component` :type "PrimitiveComponent Object Reference"))
  (returns (ResetActor :type Boolean))
  (bind _asbp_column_sensor (cast `/Game/Ruinas/Blueprints/BP_Column_Sensor` ActorInMemory)
    (:`then`
      (cast `/Game/Ruinas/Blueprints/BP_Column_Sensor` `Hit Actor`
        (:`then`
          _)
        (:`CastFailed`
          (`/Game/Ruinas/Blueprints/BPI_SetState.Toggle State` _asbp_column_sensor false)
          (return true))))
    (:`CastFailed`
      (bind _asbp_reflection (cast `/Game/Ruinas/Blueprints/BP_Reflection` ActorInMemory)
        (:`then`
          (if (or (!= `Hit Actor` _asbp_reflection) (!= (`.ReturnValue` (`PrimitiveComponent.GetMaterialFromCollisionFaceIndex` `Hit Component` 0)) (select `int` (`KismetMathLibrary.SelectInt` 0 1 (== (`GameplayStatics.GetObjectClass` ActorInMemory) "/Game/Ruinas/Blueprints/BP_LaserDuplicator.BP_LaserDuplicator_C")) :`0` "/Game/Ruinas/Assets/espejo3/M_espejo3_4.M_espejo3_4" :`1` "/Game/Ruinas/Assets/espejo1/M_espejo1_3.M_espejo1_3" :!type "Object Object Reference")))
            (`self.Desarmar` _asbp_reflection (`/Game/Ruinas/Blueprints/BP_Reflection.Id_Rayo` _asbp_reflection))
            (return true)
            (else
              _)))
        (:`CastFailed`
          _))))
  (return false))