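; Interactable lever in the Ruinas area that lowers the rising sand when the player uses it.
; Entering its box trigger binds LowerSand to the third-person character's interact press and shows the interaction widget; leaving reverses both.
; LowerSand finds all Reaching_Sand_BP actors but calls ResetSand only on the first before breaking out of the loop.
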(event `self.Box.OnComponentBeginOverlap`
  (params (OverlappedComponent :type "PrimitiveComponent Object Reference") (OtherActor :type "Actor Object Reference") (OtherComp :type "PrimitiveComponent Object Reference") (OtherBodyIndex :type Integer) (bFromSweep :type Boolean) (SweepResult :type "HitResult Structure (by ref)"))
  (bind _asthird_person_character (cast `/Game/ThirdPersonBP/Blueprints/ThirdPersonCharacter` OtherActor))
  (add `/Game/ThirdPersonBP/Blueprints/ThirdPersonCharacter.InteractPressed` _asthird_person_character (delegate `LowerSand`))
  (`/Game/ThirdPersonBP/Blueprints/ThirdPersonCharacter.ConstructInteractWidget` _asthird_person_character))

(event `LowerSand`
  (bind _outactors (`GameplayStatics.GetAllActorsOfClass` "/Game/Ruinas/Reaching_Sand_BP.Reaching_Sand_BP_C"))
  (for _array_element _outactors
    (`/Game/Ruinas/Reaching_Sand_BP.Reset Sand` _array_element)
    (break)))

(event `self.Box.OnComponentEndOverlap`
  (params (OverlappedComponent :type "PrimitiveComponent Object Reference") (OtherActor :type "Actor Object Reference") (OtherComp :type "PrimitiveComponent Object Reference") (OtherBodyIndex :type Integer))
  (bind _asthird_person_character (cast `/Game/ThirdPersonBP/Blueprints/ThirdPersonCharacter` OtherActor))
  (remove `/Game/ThirdPersonBP/Blueprints/ThirdPersonCharacter.InteractPressed` _asthird_person_character (delegate `LowerSand`))
  (`/Game/ThirdPersonBP/Blueprints/ThirdPersonCharacter.DestroyInteractionWidget` _asthird_person_character))

(fn `UserConstructionScript`)