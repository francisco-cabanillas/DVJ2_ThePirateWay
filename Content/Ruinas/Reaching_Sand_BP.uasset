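; Ruins hazard actor that raises sand from a bottom to a top height as a timed challenge once the player enters its box.
; Tick moves the sand and feeds a matching percentage to the player's Timer, stopping at either height limit.
; The trigger plays music from an offset matching current progress, so it can restart while sand is descending.
; ResetSand stops the music, lowers the sand more slowly and resets every BP_Mirror's rotation.
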(event `Reset Sand`
  (`AudioComponent.Stop` (`self.Audio`))
  (bind _output_get (set `self.move_direction` -3.0))
  (set `self.progress_bar_change` (/ (* _output_get 100.0) (- (`self.bottom_height`) (`self.top_height`))))
  (set `self.sand_moving` true)
  (bind _outactors (`GameplayStatics.GetAllActorsOfClass` "/Game/Ruinas/PuzzleLasers/BP_Mirror.BP_Mirror_C"))
  (for _array_element _outactors
    (`/Game/Ruinas/PuzzleLasers/BP_Mirror.ResetRotation` _array_element)))

(event `self.ReceiveTick`
  (params (DeltaSeconds :type "Float (single-precision)"))
  (bind _z (.z (`SceneComponent.K2_GetComponentLocation` (`self.low_sand`))))
  (if (`self.sand_moving`)
    (bind _output_get (set `self.Current_Porcentage` (+ (`self.Current_Porcentage`) (* DeltaSeconds (`self.progress_bar_change`)))))
    (`/Game/InGameOverlay/HUD_Timer.Move_Timer` (`self.Timer`) _output_get)
    (`SceneComponent.K2_SetWorldLocation` (`self.low_sand`) (`KismetMathLibrary.MakeVector` (.x (`SceneComponent.K2_GetComponentLocation` (`self.low_sand`))) (.y (`SceneComponent.K2_GetComponentLocation` (`self.low_sand`))) (+ _z (* DeltaSeconds (`self.move_direction`)))) false false)
    (if (or (> _z (`self.top_height`)) (< _z (`self.bottom_height`)))
      (set `self.sand_moving` false)
      (set `self.move_direction` 0.0))))

(event `self.Box.OnComponentBeginOverlap`
  (params (OverlappedComponent :type "PrimitiveComponent Object Reference") (OtherActor :type "Actor Object Reference") (OtherComp :type "PrimitiveComponent Object Reference") (OtherBodyIndex :type Integer) (bFromSweep :type Boolean) (SweepResult :type "HitResult Structure (by ref)"))
  (bind _move_direction (`self.move_direction`))
  (bind _sand_moving (`self.sand_moving`))
  (if (or (and (not _sand_moving) (== _move_direction 0.0)) (and _sand_moving (< _move_direction 0.0)))
    (bind _asthird_person_character (cast `/Game/ThirdPersonBP/Blueprints/ThirdPersonCharacter` OtherActor))
    (set `self.player` _asthird_person_character)
    (set `self.sand_moving` true)
    (bind _returnvalue (`GameplayStatics.CreateSound2D` "/Game/Sound/music_ruinas_Cue.music_ruinas_Cue" 1.0 1.0 0.0 null))
    (bind _output_get (set `self.Audio` _returnvalue))
    (`AudioComponent.Play` _output_get (/ (* 300.0 (`KismetMathLibrary.Abs` (- (`self.Current_Porcentage`) 100.0))) 100.0))
    (bind _output_get_2 (set `self.move_direction` 10.0))
    (set `self.Timer` (`/Game/ThirdPersonBP/Blueprints/ThirdPersonCharacter.Timer` _asthird_person_character))
    (set `self.progress_bar_change` (/ (* _output_get_2 100.0) (- (`self.bottom_height`) (`self.top_height`))))))

(fn `UserConstructionScript`)